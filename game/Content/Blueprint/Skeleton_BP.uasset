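; Skeleton enemy character with a flipbook sprite that walks along the X axis in a randomly chosen starting direction.
; Tick feeds constant movement input, and capsule hits on anything but the player reverse direction and mirror the sprite's X scale, debounced by a DoOnce reset after a short delay.
; Damage reduces health initialized from DefaultHealth; at zero it plays the death flipbook once flagged dead, though movement input continues.
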(event OnComponentHit(CapsuleComponent)
  (params (HitComponent :type Primitive%20Component%20Object%20Reference) (OtherActor :type Actor%20Object%20Reference) (OtherComp :type Primitive%20Component%20Object%20Reference) (NormalImpulse :type Vector :default "0, 0, 0") (Hit :type Hit%20Result%20Structure%20%28by%20ref%29))
  (bind _sprite (Variables|Default|GetSprite))
  (bind _returnvalue (Transformation|GetWorldScale _sprite))
  (if (!= OtherActor (Game|Player|GetPlayerPawn 0))
    (if (or (!= (.X (Math|Vector|BreakVector (.normal Hit))) 0.0) (== (.X (Math|Vector|BreakVector (.normal Hit))) (.x (Transformation|GetVelocity))))
      (Utilities|FlowControl|DoOnce false
        (:Completed
          (Variables|Default|SetSMoveRight (not (Variables|Default|GetSMoveRight)))
          (Transformation|SetWorldScale3D (Variables|Default|GetSprite) (Math|Vector|MakeVector (* (Math|Float|Absolute(Float) (.x _returnvalue)) (select (Variables|Default|GetSMoveRight) 1.0 -1.0)) (.y _returnvalue) (.z _returnvalue)))
          (Utilities|FlowControl|Delay 0.2)
          (CallFunction|ResetDirectionChangeCheck))))))

(event Custom|ResetDirectionChangeCheck
  (bind _sprite (Variables|Default|GetSprite))
  (bind _returnvalue (Transformation|GetWorldScale _sprite))
  (Utilities|FlowControl|DoOnce false) ; enters at Reset
)

(event EventTick
  (params (DeltaSeconds :type Float%20%28single-precision%29))
  (Pawn|Input|AddMovementInput "1.000000, 0, 0" (select (Variables|Default|GetSMoveRight) 1.0 -1.0) false))

(event EventBeginPlay
  (bind _sprite (Variables|Default|GetSprite))
  (bind _returnvalue (Transformation|GetWorldScale _sprite))
  (Variables|Default|SetSMoveRight (Math|Random|RandomBool))
  (Transformation|SetWorldScale3D (Variables|Default|GetSprite) (Math|Vector|MakeVector (* (.x _returnvalue) (select (Variables|Default|GetSMoveRight) 1.0 -1.0)) (.y _returnvalue) (.z _returnvalue))))

(event Game|Damage|EventAnyDamage
  (params (Damage :type Float%20%28single-precision%29) (DamageType :type Damage%20Type%20Object%20Reference) (InstigatedBy :type Controller%20Object%20Reference) (DamageCauser :type Actor%20Object%20Reference))
  (Variables|Default|SetEnemyHealth (Math|Float|Clamp(Float) (- (Variables|Default|GetEnemyHealth) Damage) 0.0 (Variables|Default|GetDefaultHealth)))
  (if (and (<= (Variables|Default|GetEnemyHealth) 0.0) (not (Variables|Default|GetIsDead)))
    (Variables|Default|SetIsDead true)
    (CallFunction|EnemyDied)))

(fn ConstructionScript
  (Variables|Default|SetEnemyHealth (Variables|Default|GetDefaultHealth)))

(fn EnemyDied
  (Sprite|SetFlipbook (Variables|Default|GetSprite) "/Game/Assets/Flipbooks/FB_SkeletonDeath.FB_SkeletonDeath"))