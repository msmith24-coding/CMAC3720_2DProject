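; Child Blueprint of a wizard enemy, using a Paper2D sprite, whose death ends the game.
; The EnemyDied override calls the parent, sets the death flipbook, then immediately destroys the actor and opens the EndGame_M level, with no delay for the animation.
; Tick adds zero-vector movement input, so it contributes no motion, and the construction script only calls the parent.
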(event EventBeginPlay
  (|CallParentFunction) ; This node is disabled and will not be called.\nDrag off pins to build functionality.
)

(event Collision|EventActorBeginOverlap
  (params (OtherActor :type Actor%20Object%20Reference)))

(event EventTick
  (params (DeltaSeconds :type Float%20%28single-precision%29))
  (Pawn|Input|AddMovementInput "0, 0, 0" 1.0 false))

(fn ConstructionScript
  (|CallParentFunction))

(fn EnemyDied
  (|CallParentFunction)
  (Sprite|SetFlipbook (Variables|Default|GetSprite) "/Game/Assets/Flipbooks/FB_WizardDeath.FB_WizardDeath")
  (Actor|DestroyActor)
  (Game|OpenLevel(byName) "EndGame_M"))